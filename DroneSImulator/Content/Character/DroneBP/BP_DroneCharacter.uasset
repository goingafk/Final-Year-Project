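; Drone character prototype that moves vertically on physics thrust, with a placeholder Cube standing in for the future model.
; On BeginPlay it shifts the Cube's centre of mass in local X and Y toward the PhysicsThruster's position.
; The Move_Up axis sets thrust strength as scaled input plus a constant baseline.
; A control-rotation-based AddMovementInput chain is left disconnected and never runs.
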(event EventBeginPlay
  (bind _physicsthruster (Variables|Default|GetPhysicsThruster))
  (bind _cube (Variables|Default|GetCube))
  (bind _cube_2 (Variables|Default|GetCube))
  (bind _returnvalue (Transformation|GetWorldLocation _physicsthruster))
  (bind _returnvalue_2 (Physics|GetCenterOfMass _cube_2 "None"))
  (bind _returnvalue_3 (Transformation|GetWorldRotation _cube))
  (bind _returnvalue_4 (Class|KismetMathLibrary|NegateRotator _returnvalue_3))
  (bind _returnvalue_5 (- _returnvalue _returnvalue_2))
  (bind _returnvalue_6 (Math|Vector|RotateVector _returnvalue_5 _returnvalue_4))
  ;[1 1 1] Setting the centre of mass to where the physics thruster
  (Class|PrimitiveComponent|SetCenterOfMass (Variables|Default|GetCube) (Math|Vector|MakeVector (.x _returnvalue_6) (.y _returnvalue_6) 0.0) "None"))

(event Input|AxisEvents|InputAxisMove_Up
  (params (AxisValue :type Float%20%28single-precision%29))
  (Variables|/Script/Engine.PhysicsThrusterComponent|SetThrustStrength (Variables|Default|GetPhysicsThruster) (+ (* AxisValue 1e+04) 9.7e+02)))

(fn ConstructionScript)